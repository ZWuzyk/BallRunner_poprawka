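; BP_WinVolume is a level-exit volume that reacts when the player overlaps it, gated on the crystals left on the map.
; CheckForCrystals counts BP_crystal actors and passes when two or fewer remain.
; A Polish debug message announces either a new level or remaining crystals.
; On success it calls CompleteLevel, which is unfinished: it only reads the current level name, leaving the LevelNames lookup unconnected.
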(event `self.ReceiveActorBeginOverlap`
  (params (OtherActor :type "Actor Object Reference"))
  (`/Game/Blueprints/Libraries/ML_Actors.IsPlayer` OtherActor
    (:`IsPlayer`
      (if (`self.CheckForCrystals`)
        (`KismetSystemLibrary.PrintString` "Nowy poziom!!!")
        (`self.Complete Level`)
        (else
          (`KismetSystemLibrary.PrintString` "Na mapie są jeszcze kryształy!"))))))

(fn `CheckForCrystals`
  (returns (`Return Value` :type Boolean))
  (bind _outactors (`GameplayStatics.GetAllActorsOfClass` "/Game/Blueprints/Actors/Collectables/BP_crystal.BP_crystal_C"))
  (return (>= 2 (`KismetArrayLibrary.Array_Length` _outactors))))

(fn `Complete Level`
  (bind _returnvalue (`GameplayStatics.GetCurrentLevelName` true)))

(fn `UserConstructionScript`)