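; BP_Projectile is a projectile actor that damages the player pawn on contact.
; When its collision sphere begins an overlap, it applies damage and prints a debug string only if the other actor is player 0's pawn.
; Any overlap destroys the collision and Sphere components, leaving the actor itself in place.
; The graph contains no movement or spawning logic, and the construction script is empty.
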(event `self.sphere_collission.OnComponentBeginOverlap`
  (params (OverlappedComponent :type "PrimitiveComponent Object Reference") (OtherActor :type "Actor Object Reference") (OtherComp :type "PrimitiveComponent Object Reference") (OtherBodyIndex :type Integer) (bFromSweep :type Boolean) (SweepResult :type "HitResult Structure (by ref)"))
  (if (!= OtherActor (`GameplayStatics.GetPlayerPawn` 0))
    (`ActorComponent.K2_DestroyComponent` (`self.sphere_collission`))
    (`ActorComponent.K2_DestroyComponent` (`self.Sphere`))
    (else
      (`GameplayStatics.ApplyDamage` (`GameplayStatics.GetPlayerPawn` 0) 1.0)
      (`KismetSystemLibrary.PrintString` "DAMAGE ŁeŁO ŁEŁO" true false)
      (`ActorComponent.K2_DestroyComponent` (`self.sphere_collission`))
      (`ActorComponent.K2_DestroyComponent` (`self.Sphere`)))))

(fn `UserConstructionScript`)