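; BP_cannon is an automatic cannon actor that fires BP_Projectile actors indefinitely, with no aiming or trigger logic.
; After an initial delay on BeginPlay, it enters a latent Delay loop paced by the FireRate variable, which acts as the interval between shots.
; Each shot always spawns at the Arrow component's world location and rotation, uniformly scaled by ProjectileScale.
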(event `self.ReceiveBeginPlay`
  (`KismetSystemLibrary.Delay` 4.0)
  (`KismetSystemLibrary.Delay` (`self.Fire Rate`) :!label _label)
  (`|SpawnActorFromClass` "/Game/Blueprints/Actors/Projectiles/BP_Projectile.BP_Projectile_C" (`KismetMathLibrary.MakeTransform` (`SceneComponent.K2_GetComponentLocation` (`self.Arrow`)) (`SceneComponent.K2_GetComponentRotation` (`self.Arrow`)) (`KismetMathLibrary.Conv_DoubleToVector` (`self.Projectile Scale`))) "AlwaysSpawn" "OverrideRootScale" null null)
  (goto _label))

(fn `UserConstructionScript`)