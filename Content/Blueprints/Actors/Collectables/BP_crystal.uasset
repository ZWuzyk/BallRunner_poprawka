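; BP_crystal is a collectable crystal that gets pulled into the player when touched, then disappears.
; On overlap with player pawn 0 it stores its starting location, scale and light intensity, then plays a timeline.
; The timeline's curves lerp it toward the player's live position while shrinking it and fading its point light to zero.
; The actor destroys itself when the timeline finishes, with no score or pickup effect applied here.
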(event `self.ReceiveActorBeginOverlap`
  (params (OtherActor :type "Actor Object Reference"))
  (`self.IsPlayer` OtherActor
    (:`IsPlayer`
      (`self.SetStartValues`)
      (bind (_direction _smoothlerpalpha _scale_in_time _intensity_in_time) (`Timeline|Timeline_0`)
        (:`Update`
          (`self.ChangeLocation` _smoothlerpalpha)
          (`self.Change Scale` _scale_in_time)
          (`self.Change Intensity` _intensity_in_time))
        (:`Finished`
          (`self.K2_DestroyActor`))))))

(fn `Change Intensity`
  (params (Alpha :type "Float (double-precision)"))
  (`LightComponent.SetIntensity` (`self.PointLight`) (`KismetMathLibrary.Lerp` (`self.Lerp Start Intensity`) 0.0 Alpha)))

(fn `Change Scale`
  (params (Alpha :type "Float (double-precision)"))
  (`self.SetActorScale3D` (`KismetMathLibrary.VLerp` (`self.Lerp Start Scale`) (0.0 0.0 0.0) Alpha)))

(fn `ChangeLocation`
  (params (Alpha :type "Float (double-precision)"))
  (`self.K2_SetActorLocation` (`KismetMathLibrary.VLerp` (`self.Lerp Start Location`) (`self.K2_GetActorLocation` (`GameplayStatics.GetPlayerPawn` 0)) Alpha)))

(fn `SetStartValues`
  (set `self.Lerp Start Location` (`self.K2_GetActorLocation`))
  (set `self.Lerp Start Scale` (`self.GetActorScale3D`))
  (set `self.Lerp Start Intensity` (`LightComponentBase.Intensity` (`self.PointLight`))))

(fn `UserConstructionScript`)